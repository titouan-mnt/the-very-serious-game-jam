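; AI controller for a bot on BP_ThirdPersonCharacter pawns, currently inert because every event is empty and all logic sits in disconnected chains.
; The unwired drafts find the nearest other character, move toward it with AIMoveTo and call TryGrab.
; Other orphaned fragments branch on IsHolding to HandleHolding or FindTarget, start a looping think timer, aim control rotation at the target and set ThrowStrength, alongside debug prints.
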(event Custom|UpdateTarget)

(event Custom|BotThink)

(event Custom|HandleHolding)

(event Custom|FindTarget)

(event EventBeginPlay)

(event EventTick
  (params (DeltaSeconds :type Float%20%28single-precision%29)))

(fn ConstructionScript)